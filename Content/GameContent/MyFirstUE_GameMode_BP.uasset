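; Game mode Blueprint that tracks how many cars are inside and decides whether the player has won or lost.
; AddCar and RemoveCar events raise or lower the current count, then share one check against the total number of cars needed to win.
; Every change immediately prints a Spanish win message in green or a lose message in red, so losing shows whenever the count is below target.
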(event Custom|AddCar
  (Math|Integer|IncrementInt (Variables|Default|GetCurrentCarsInside)
    (:%20%20
      (if (>= (Variables|Default|GetCurrentCarsInside) (Variables|Default|GetTotalNumCarToWin))
        (Development|PrintString "Has ganado" true true "(R=0.170675,G=1.000000,B=0.000000,A=1.000000)")
        (else
          (Development|PrintString "Has perdido" true true "(R=1.000000,G=0.008232,B=0.000000,A=1.000000)"))))))

(event Custom|RemoveCar
  (Math|Integer|DecrementInt (Variables|Default|GetCurrentCarsInside)
    (:%20%20
      (if (>= (Variables|Default|GetCurrentCarsInside) (Variables|Default|GetTotalNumCarToWin))
        (Development|PrintString "Has ganado" true true "(R=0.170675,G=1.000000,B=0.000000,A=1.000000)")
        (else
          (Development|PrintString "Has perdido" true true "(R=1.000000,G=0.008232,B=0.000000,A=1.000000)"))))))

(fn ConstructionScript)