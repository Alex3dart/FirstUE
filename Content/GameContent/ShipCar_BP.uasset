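; ShipCar_BP is a player-controlled vehicle pawn driven by input axes, with a spring-arm camera.
; Vertical and horizontal move axes feed AddMovementInput along the actor's forward and right vectors, so horizontal input strafes rather than steers.
; Mouse axes add controller pitch and yaw, while the wheel zooms by changing the spring arm's length with no clamp.
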(event Input|AxisEvents|InputAxisMouseHorizontal
  (params (AxisValue :type Float%20%28single-precision%29))
  ;[0 0.00901 1 1 50] Controles Mouse
  ;;[1 1 1 1 30] Rotacion Camara
  (Pawn|Input|AddControllerYawInput AxisValue))

(event Input|AxisEvents|InputAxisMouseVertical
  (params (AxisValue :type Float%20%28single-precision%29))
  ;[0 0.00901 1 1 50] Controles Mouse
  ;;[1 1 1 1 30] Rotacion Camara
  (Pawn|Input|AddControllerPitchInput AxisValue))

(event Input|AxisEvents|InputAxisMoveHorizontal
  (params (AxisValue :type Float%20%28single-precision%29))
  ;[1 1 1 1 50] MOVIMIENTO DEL COCHE
  (Pawn|Input|AddMovementInput (Transformation|GetActorRightVector) AxisValue false))

(event Input|AxisEvents|InputAxisMoveVertical
  (params (AxisValue :type Float%20%28single-precision%29))
  ;[1 1 1 1 50] MOVIMIENTO DEL COCHE
  (Pawn|Input|AddMovementInput (Transformation|GetActorForwardVector) AxisValue false))

(event Input|AxisEvents|InputAxisMouseWheel
  (params (AxisValue :type Float%20%28single-precision%29))
  (bind _springarm (Variables|Default|GetSpringArm))
  ;[0 0.00901 1 1 50] Controles Mouse
  ;;[1 1 1 1 30] ZOOM DE CAMARA
  (Variables|/Script/Engine.SpringArmComponent|SetTargetArmLength _springarm (+ (* AxisValue 5.0) (Variables|/Script/Engine.SpringArmComponent|GetTargetArmLength _springarm))))

(fn ConstructionScript)